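; Character Blueprint for Maestra, the classical fighter, scripting cinematic setup and move-specific presentation.
; Her super attack blacks out the stage by hiding lights, sky, fog and name-prefix-matched meshes, then spawns a spotlight and ghost trail.
; It also slows the opponent and blends between finale cameras, restoring camera and scenery after delays.
; Other state changes stop the trail, with timed bow or sword visibility swaps for certain attacks.
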(event EventBPEventsonStateBegin
  (params (state :type Data%20Table%20Row%20Handle%20Structure))
  (bind _rowname (Utilities|Struct|BreakDataTableRowHandle state))
  (if (Utilities|Name|Equal(Name) _rowname "MaestraSuperAttack")
    (bind _opponent (CallFunction|GetOpponent2))
    (Utilities|FlowControl|Sequence
      (:then_0
        (bind _outactors (Actor|GetAllActorsOfClass "/Script/Engine.SkyLight"))
        (Rendering|SetActorHiddenInGame (Utilities|Array|Get(acopy) _outactors) true))
      (:then_1
        (bind _returnvalue (Game|SpawnActorfromClass "/Game/BPs/World/PlayerSpotlight_Super.PlayerSpotlight_Super_C" (Math|Transform|MakeTransform "0,20.000000,-10.000000") "Undefined" 0 0))
        (bind _returnvalue_2 (Class|FighterCharacter|GetIndex))
        (Variables|/Game/BPs/World/PlayerSpotlight_Super.PlayerSpotlight_Super_C|Setplayer _returnvalue _returnvalue_2)
        (Variables|/Script/Engine.Actor|SetCustomTimeDilation _opponent 0.001)
        (CallFunction|SpawnGhostTrail)
        (Game|Player|SetViewTargetwithBlend (Game|GetPlayerController 0) (Variables|/Script/Engine.ChildActorComponent|GetChildActor (Variables|Default|GetFinaleCamera1)) 0.0 "VTBlend_Linear" 0.0 false)
        (Game|Player|SetViewTargetwithBlend (Game|GetPlayerController 0) (Variables|/Script/Engine.ChildActorComponent|GetChildActor (Variables|Default|GetFinaleCamera2)) 2.5 "VTBlend_Linear" 0.0 false)
        (Utilities|FlowControl|Delay 1.0)
        (Variables|/Script/Engine.Actor|SetCustomTimeDilation _opponent 0.6)
        (bind _asbbgame_state (Utilities|Casting|CastToBBGameState (Game|GetGameState)))
        (Game|Player|SetViewTargetwithBlend (Game|GetPlayerController 0) (Variables|/Script/BeatBoxers.BBGameState|GetMainCamera _asbbgame_state) 0.0 "VTBlend_Linear" 0.0 false)
        (Utilities|FlowControl|Delay 3.5)
        (Utilities|FlowControl|Sequence
          (:then_0
            (bind _outactors_2 (Actor|GetAllActorsOfClass "/Script/Engine.SkyLight"))
            (Rendering|SetActorHiddenInGame (Utilities|Array|Get(acopy) _outactors_2) false))
          (:then_1
            (bind _outactors_3 (Actor|GetAllActorsOfClass "/Script/Engine.AtmosphericFog"))
            (Rendering|SetActorHiddenInGame (Utilities|Array|Get(acopy) _outactors_3) false))
          (:then_2
            (bind _outactors_4 (Actor|GetAllActorsOfClass "/Script/Engine.ExponentialHeightFog"))
            (Rendering|SetActorHiddenInGame (Utilities|Array|Get(acopy) _outactors_4) false))
          (:then_3
            (bind _outactors_5 (Actor|GetAllActorsOfClass "/Script/Engine.StaticMeshActor"))
            (for _array_element _outactors_5
              (if (Math|Boolean|ORBoolean (Utilities|Enum|Equal(Enum) (Utilities|String|GetSubstring (Utilities|GetDisplayName _array_element) 0 12) "RikiBuilding") (Utilities|Enum|Equal(Enum) (Utilities|String|GetSubstring (Utilities|GetDisplayName _array_element) 0 3) "do_") (Utilities|Enum|Equal(Enum) (Utilities|String|GetSubstring (Utilities|GetDisplayName _array_element) 0 10) "falt_plane"))
                (Rendering|SetActorHiddenInGame _array_element false))))
          (:then_4
            (bind _outactors_6 (Actor|GetAllActorsOfClass "/Engine/EngineSky/BP_Sky_Sphere.BP_Sky_Sphere_C"))
            (Rendering|SetActorHiddenInGame (Utilities|Array|Get(acopy) _outactors_6) false))
          (:then_5
            (bind _outactors_7 (Actor|GetAllActorsOfClass "/Script/Engine.Light"))
            (for _array_element_2 _outactors_7
              (Rendering|SetActorHiddenInGame _array_element_2 false)))
          (:then_6
            (bind _outactors_8 (Actor|GetAllActorsOfClass "/Game/BPs/World/StadiumLights.StadiumLights_C"))
            (for _array_element_3 _outactors_8
              (Rendering|SetActorHiddenInGame _array_element_3 false)))
          (:then_7
            (Actor|DestroyActor _returnvalue))))
      (:then_2
        (bind _outactors_9 (Actor|GetAllActorsOfClass "/Script/Engine.AtmosphericFog"))
        (Rendering|SetActorHiddenInGame (Utilities|Array|Get(acopy) _outactors_9) true))
      (:then_3
        (bind _outactors_10 (Actor|GetAllActorsOfClass "/Script/Engine.ExponentialHeightFog"))
        (Rendering|SetActorHiddenInGame (Utilities|Array|Get(acopy) _outactors_10) true))
      (:then_4
        (bind _outactors_11 (Actor|GetAllActorsOfClass "/Script/Engine.StaticMeshActor"))
        (for _array_element_4 _outactors_11
          (if (Math|Boolean|ORBoolean (Utilities|Enum|Equal(Enum) (Utilities|String|GetSubstring (Utilities|GetDisplayName _array_element_4) 0 12) "RikiBuilding") (Utilities|Enum|Equal(Enum) (Utilities|String|GetSubstring (Utilities|GetDisplayName _array_element_4) 0 3) "do_") (Utilities|Enum|Equal(Enum) (Utilities|String|GetSubstring (Utilities|GetDisplayName _array_element_4) 0 10) "falt_plane"))
            (Rendering|SetActorHiddenInGame _array_element_4 true))))
      (:then_5
        (bind _outactors_12 (Actor|GetAllActorsOfClass "/Engine/EngineSky/BP_Sky_Sphere.BP_Sky_Sphere_C"))
        (Rendering|SetActorHiddenInGame (Utilities|Array|Get(acopy) _outactors_12) true))
      (:then_6
        (bind _outactors_13 (Actor|GetAllActorsOfClass "/Script/Engine.Light"))
        (for _array_element_5 _outactors_13
          (Rendering|SetActorHiddenInGame _array_element_5 true)))
      (:then_7
        (bind _outactors_14 (Actor|GetAllActorsOfClass "/Game/BPs/World/StadiumLights.StadiumLights_C"))
        (for _array_element_6 _outactors_14
          (Rendering|SetActorHiddenInGame _array_element_6 true))))
    (else
      (CallFunction|StopGhostTrail)
      (if (Math|Boolean|ORBoolean (Utilities|Name|Equal(Name) _rowname "MaestraSpecialAttack3") (Utilities|Name|Equal(Name) _rowname "MaestraSpecialAttack3OffBeat") (Utilities|Name|Equal(Name) _rowname "MaestraSpecialAttack3Air") (Utilities|Name|Equal(Name) _rowname "MaestraSpecialAttack3OffBeatAir"))
        (Development|SetHiddeninGame (Variables|Default|Getbow) false false)
        (Utilities|FlowControl|Delay 0.7)
        (Development|SetHiddeninGame (Variables|Default|Getbow) true false)
        (elif (or (Utilities|Name|Equal(Name) _rowname "MaestraLightAttack") (Utilities|Name|Equal(Name) _rowname "MaestraLightAttackOffBeat"))
          (Development|SetHiddeninGame (Variables|Default|Getsword) true false)
          (Development|SetHiddeninGame (Variables|Default|GetHiddenSword2) false false)
          (Utilities|FlowControl|Delay 0.5)
          (Development|SetHiddeninGame (Variables|Default|Getsword) false false)
          (Development|SetHiddeninGame (Variables|Default|GetHiddenSword2) true false))))))

(event EventBeginPlay
  (|CallParentFunction)
  (CallFunction|CinematicSetup))

(fn ConstructionScript
  (|CallParentFunction))

(fn CinematicSetup
  (Variables|Default|SetWCinematic1 "/Game/Assets/Characters/Classical/Animations/char_classical_anim_walk_v01_Montage.char_classical_anim_walk_v01_Montage")
  (Variables|Default|SetWCinematic2 "/Game/Assets/ToBeOrganized/Character/ToBeReplaced/Marth/Animations/Montages/AppealHi_8Sec_Montage.AppealHi_8Sec_Montage")
  (Variables|Default|SetWCinematic3 "/Game/Assets/Characters/Rock/Animations/char_rock_anim_block_v01_Montage.char_rock_anim_block_v01_Montage")
  (Variables|Default|SetWCinematic4 0)
  (Variables|Default|SetLCinematic "/Game/Assets/Characters/Classical/Animations/char_classical_anim_stagger_v01_Anim_Montage.char_classical_anim_stagger_v01_Anim_Montage")
  (Variables|Default|SetCinematicHitFX "/Game/Assets/Characters/Classical/Particles/Characters_Class_VFX_SUPERHit.Characters_Class_VFX_SUPERHit"))