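; Blueprint for the rock fighter Riff, layering effects onto combat states and setting up cinematic assets.
; The super attack darkens the stage by hiding actors, spawns a spotlight, slows the opponent and blends to a spawned camera, playing a Level Sequence if the opponent is stunned, then restores music volume.
; Crouch and dashes show timed guitar props or dash-cancel FX.
; Blocking shows shield effects only when on beat.
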(event Collision|EventActorBeginOverlap
  (params (OtherActor :type Actor%20Object%20Reference))
  (|CallParentFunction OtherActor))

(event EventBPEventsonStateBegin
  (params (state :type Data%20Table%20Row%20Handle%20Structure))
  (bind _rowname (Utilities|Struct|BreakDataTableRowHandle state))
  (bind _returnvalue (Transformation|GetActorLocation))
  (bind _guitar_for_slide (Variables|Default|Getguitar%20for%20slide))
  (bind _mesh (Variables|Character|GetMesh))
  (bind _returnvalue_2 (Transformation|GetWorldTransform _mesh))
  (bind (_x _y _z) (Math|Vector|BreakVector _returnvalue))
  (bind (_location _rotation _scale) (Math|Transform|BreakTransform _returnvalue_2))
  (if (Utilities|Name|Equal(Name) _rowname "RiffSuperAttack")
    (bind _opponent (CallFunction|GetOpponent2))
    (Utilities|FlowControl|Sequence
      (:then_0
        (|darkenthelights_2))
      (:then_1
        (bind _returnvalue_3 (|makespotlight_2))
        (Variables|/Script/Engine.Actor|SetCustomTimeDilation _opponent 0.001)
        (CallFunction|SpawnGhostTrail)
        (bind _returnvalue_4 (Game|SpawnActorfromClass "/Script/Engine.CameraActor" (Math|Transform|MakeTransform (Math|Vector|MakeVector _x 5e+02 _z) "0.000000,-90.000000, 0" "1,1,1") "Undefined" 0 0))
        (Camera|SetFieldOfView (Variables|/Script/Engine.CameraActor|GetCameraComponent _returnvalue_4) 5e+01)
        (Game|Player|SetViewTargetwithBlend (Game|GetPlayerController 0) _returnvalue_4 0.8 "VTBlend_Linear" 0.0 false)
        (Utilities|FlowControl|Delay 0.5)
        (Variables|/Script/Engine.Actor|SetCustomTimeDilation _opponent 1.0)
        (bind _asbbgame_state (Utilities|Casting|CastToBBGameState (Game|GetGameState)))
        (Game|Player|SetViewTargetwithBlend (Game|GetPlayerController 0) (Variables|/Script/BeatBoxers.BBGameState|GetMainCamera _asbbgame_state) 0.0 "VTBlend_Linear" 0.0 false)
        (Utilities|FlowControl|Delay 0.3)
        (CallFunction|StopGhostTrail)
        (if (Class|FighterCharacter|IsStunned _opponent)
          (Utilities|FlowControl|Sequence
            (:then_0
              (|brightenthelights_2_2_2 _returnvalue_3
                (:then_8
                  (bind _returnvalue_5 (Sequencer|Player|CreateLevelSequencePlayer "/Game/Cinematics/Riff/Riff_Super/RiffSuper_Master.RiffSuper_Master"))
                  (Sequencer|Player|Play _returnvalue_5 :!class /Script/MovieScene.MovieSceneSequencePlayer)
                  (Utilities|FlowControl|Delay 7.4)
                  (Utilities|FlowControl|Sequence :!label _label
                    (:then_0
                      (Rendering|SetActorHiddenInGame false)
                      (Rendering|SetActorHiddenInGame _opponent false))
                    (:then_1
                      (bind _newtrack_0 (Timeline|Timeline_3 PlayFromStart)
                        (:Update
                          (Class|FMODAudioComponent|SetVolume (Variables|/Game/BPs/MyBasicMusicBox.MyBasicMusicBox_C|GetFMODAudio (Utilities|Array|Get(acopy) (stale _outactors))) _newtrack_0))))))))
            (:then_1
              (Rendering|SetActorHiddenInGame true)
              (Rendering|SetActorHiddenInGame _opponent true)))
          (else
            (|brightenthelights_2_2 _returnvalue_3
              (:then_8
                (goto _label))))))
      (:then_2
        (bind _outactors (Actor|GetAllActorsOfClass "/Game/BPs/MyBasicMusicBox.MyBasicMusicBox_C"))
        (Class|FMODAudioComponent|SetVolume (Variables|/Game/BPs/MyBasicMusicBox.MyBasicMusicBox_C|GetFMODAudio (Utilities|Array|Get(acopy) _outactors)) 0.2)))
    (elif (Utilities|Name|Equal(Name) _rowname "RiffCrouchAttack")
      (Development|SetHiddeninGame (Variables|Default|Getchar_rock_obj_guitar_v1) false false)
      (Timeline|Timeline_2 PlayFromStart
        (:Finished
          (Development|SetHiddeninGame (Variables|Default|Getchar_rock_obj_guitar_v1) true false)))
      (elif (Utilities|Name|Equal(Name) _rowname "RiffDashForward")
        (Development|SetHiddeninGame _guitar_for_slide false false :!label _label_2)
        (Timeline|hide%20guitar PlayFromStart
          (:Finished
            (Development|SetHiddeninGame _guitar_for_slide true false)))
        (elif (Utilities|Name|Equal(Name) _rowname "RiffDashCancelForward")
          (Utilities|FlowControl|Sequence
            (:then_0
              (goto _label_2))
            (:then_1
              (Game|SpawnActorfromClass "/Game/Assets/Characters/Shared/Effects/dashCancelFx.dashCancelFx_C" (Math|Transform|MakeTransform (+ _location (Math|Vector|RotateVector (* (Transformation|GetActorForwardVector (Pawn|GetViewTarget (Game|GetPlayerController 0))) 1e+01) (Math|Rotator|MakeRotator 0.0 0.0 (+ (.Yaw (Math|Rotator|BreakRotator (Camera|GetCameraRotation (Game|GetPlayerCameraManager 0)))) 5e+01)))) _rotation _scale) "Undefined" 0 0 :!label _label_3)))
          (elif (Utilities|Name|Equal(Name) _rowname "RiffDashCancelBackward")
            (goto _label_3)))))))

(event EventTick
  (params (DeltaSeconds :type Float%20%28single-precision%29))
  (|CallParentFunction DeltaSeconds))

(event EventChangebalance
  (bind _outactors (Actor|GetAllActorsOfClass "/Game/BPs/MyBasicMusicBox.MyBasicMusicBox_C"))
  (Class|FMODAudioComponent|SetParameter (Variables|/Game/BPs/MyBasicMusicBox.MyBasicMusicBox_C|GetFMODAudio (Utilities|Array|Get(acopy) _outactors)) "balance" 0.0))

(event EventBeginPlay
  (|CallParentFunction)
  (CallFunction|CinematicSetup))

(event EventBlockEffects
  ;[1 1 1] Blocking Effects Logic
  (Variables|Default|Setblocking true)
  (bind _outactors (Actor|GetAllActorsOfClass "/Game/BPs/MyBasicMusicBox.MyBasicMusicBox_C"))
  (bind _asmy_bbgame_mode (Utilities|Casting|CastToMyBBGameMode (Game|GetGameMode)))
  (bind _returnvalue (Class|BBGameMode|IsonBeat _asmy_bbgame_mode (Class|BasicMusicBox|GetBeatAccuracy (Utilities|Array|Get(acopy) _outactors))))
  (if _returnvalue
    (Rendering|SetRenderCustomDepth (Variables|Character|GetMesh) true)
    (Effects|SpawnEmitterAttached "/Game/Assets/Characters/Rock/Particles/Characters_Shared_VFX_Shield_Riff.Characters_Shared_VFX_Shield_Riff" (Variables|Default|GetCapsuleComponent) "None")))

(event EventStopBlockEffects
  ;[1 1 1] Blocking Effects Logic
  (Variables|Default|Setblocking false)
  (Rendering|SetRenderCustomDepth (Variables|Character|GetMesh) false))

(fn ConstructionScript
  (|CallParentFunction))

(fn CinematicSetup
  (Variables|Default|SetWCinematic1 0)
  (Variables|Default|SetWCinematic2 0)
  (Variables|Default|SetWCinematic3 0)
  (Variables|Default|SetWCinematic4 0)
  (Variables|Default|SetLCinematic "/Game/Assets/Characters/Rock/Animations/char_rock_anim_stagger_v01_Montage.char_rock_anim_stagger_v01_Montage")
  (Variables|Default|SetCinematicHitFX "/Game/Assets/Characters/Classical/Particles/Characters_Class_VFX_SUPERHit.Characters_Class_VFX_SUPERHit"))